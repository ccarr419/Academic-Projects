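; Pickup actor that grants coins, grapples or bombs to the player hero.
; On overlap with a PlayerHero it adds ItemQuantity to the matching counter on the hero, then destroys itself.
; The IsCoins and IsGrapples flags select the item type, with bombs as the fallback when both are false.
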(event EventBeginPlay)

(event Collision|EventActorBeginOverlap
  (params (OtherActor :type Actor%20Object%20Reference))
  (bind _asplayer_hero (Utilities|Casting|CastToPlayerHero OtherActor))
  (if (Variables|Default|GetisCoins)
    (Variables|/Game/Blueprints/PlayerHero/PlayerHero.PlayerHero_C|SetnumPlayerCoins _asplayer_hero (+ (Variables|Default|GetitemQuantity) (Variables|/Game/Blueprints/PlayerHero/PlayerHero.PlayerHero_C|GetnumPlayerCoins _asplayer_hero)))
    (elif (Variables|Default|GetisGrapples)
      (Variables|/Game/Blueprints/PlayerHero/PlayerHero.PlayerHero_C|SetnumPlayerGrapples _asplayer_hero (+ (Variables|Default|GetitemQuantity) (Variables|/Game/Blueprints/PlayerHero/PlayerHero.PlayerHero_C|GetnumPlayerGrapples _asplayer_hero)))
      (else
        (Variables|/Game/Blueprints/PlayerHero/PlayerHero.PlayerHero_C|SetnumPlayerBombs _asplayer_hero (+ (Variables|Default|GetitemQuantity) (Variables|/Game/Blueprints/PlayerHero/PlayerHero.PlayerHero_C|GetnumPlayerBombs _asplayer_hero))))))
  (Actor|DestroyActor))

(fn ConstructionScript)