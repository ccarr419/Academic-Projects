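; Mortise is an enemy Blueprint whose destruction triggers the level-complete screen and ends the game.
; On Destroyed, it adds a LevelComplete widget to the viewport and switches the first player controller to UI-only input focused on it.
; A three-second Delay on the actor being destroyed then leads to QuitGame.
; BeginPlay, Tick and the construction script only call the parent class.
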(event EventBeginPlay
  (|CallParentFunction))

(event Collision|EventActorBeginOverlap
  (params (OtherActor :type Actor%20Object%20Reference)))

(event EventTick
  (params (DeltaSeconds :type Float%20%28single-precision%29))
  (|CallParentFunction 0.0))

(event EventDestroyed
  (bind _returnvalue (UserInterface|CreateWidget "/Game/UMG/LevelComplete.LevelComplete_C"))
  (Input|SetInputModeUIOnly (Game|GetPlayerController 0) _returnvalue "DoNotLock")
  (UserInterface|Viewport|AddtoViewport _returnvalue 0)
  (Utilities|FlowControl|Delay 3.0)
  (Game|QuitGame 0 "Quit"))

(fn ConstructionScript
  (|CallParentFunction))