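; Wolf enemy character that specializes a parent enemy class with its own damage and handicap values.
; BeginPlay sets those two values before calling the parent's BeginPlay.
; Hit, walking off a ledge, Tick and the construction script only forward to the parent, so all other behavior is inherited.
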(event EventBeginPlay
  (Variables|Default|SetenemyDamage 1e+01)
  (Variables|Default|SetenemyHandicap 2.0)
  (|CallParentFunction))

(event EventTick
  (params (DeltaSeconds :type Float%20%28single-precision%29))
  (|CallParentFunction DeltaSeconds))

(event Collision|EventHit
  (params (MyComp :type Primitive%20Component%20Object%20Reference) (Other :type Actor%20Object%20Reference) (OtherComp :type Primitive%20Component%20Object%20Reference) (bSelfMoved :type Boolean) (HitLocation :type Vector) (HitNormal :type Vector) (NormalImpulse :type Vector) (Hit :type Hit%20Result%20Structure%20%28by%20ref%29))
  (|CallParentFunction MyComp Other OtherComp bSelfMoved HitLocation HitNormal NormalImpulse Hit))

(event EventOnWalkingOffLedge
  (params (PreviousFloorImpactNormal :type Vector%20%28by%20ref%29) (PreviousFloorContactNormal :type Vector%20%28by%20ref%29) (PreviousLocation :type Vector%20%28by%20ref%29) (TimeDelta :type Float%20%28single-precision%29))
  (|CallParentFunction PreviousFloorImpactNormal PreviousFloorContactNormal PreviousLocation TimeDelta))

(fn ConstructionScript
  (|CallParentFunction))