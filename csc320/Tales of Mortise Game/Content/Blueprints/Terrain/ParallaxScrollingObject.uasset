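; A terrain actor that creates a parallax scrolling effect by moving relative to the player hero.
; BeginPlay records its own location and the first PlayerHero's location.
; Each Tick it re-finds the hero and, when it has moved, offsets itself by the hero's X and Z movement times per-axis scale factors.
; Y stays fixed, and the hero is looked up with GetAllActorsOfClass every frame rather than cached.
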(event EventBeginPlay
  ;[1 1 1] Main
  (Variables|Default|SetthisActorsLocation (Transformation|GetActorLocation))
  (bind _outactors (Actor|GetAllActorsOfClass "/Game/Blueprints/PlayerHero/PlayerHero.PlayerHero_C"))
  (Variables|Default|SetoldPlayerLocation (Transformation|GetActorLocation (Utilities|Array|Get(acopy) _outactors))))

(event EventTick
  (params (DeltaSeconds :type Float%20%28single-precision%29))
  ;[1 1 1] Set Parallax Scrolling Scale
  (bind _outactors (Actor|GetAllActorsOfClass "/Game/Blueprints/PlayerHero/PlayerHero.PlayerHero_C"))
  (if (Utilities|IsValid (Utilities|Array|Get(acopy) _outactors))
    (bind _output_get (Variables|Default|SetnewPlayerLocation (Transformation|GetActorLocation (Utilities|Array|Get(acopy) _outactors))))
    (if (Math|Vector|NotEqual(Vector) _output_get (Variables|Default|GetoldPlayerLocation) 0.0001)
      (bind _output_get_2 (Variables|Default|SetthisActorsLocation (Math|Vector|MakeVector (+ (* (- (.X (Math|Vector|BreakVector (Variables|Default|GetnewPlayerLocation))) (.X (Math|Vector|BreakVector (Variables|Default|GetoldPlayerLocation)))) (Variables|Default|GetparallaxScrollingScaleX)) (.X (Math|Vector|BreakVector (Variables|Default|GetthisActorsLocation)))) (.Y (Math|Vector|BreakVector (Variables|Default|GetthisActorsLocation))) (+ (* (- (.Z (Math|Vector|BreakVector (Variables|Default|GetnewPlayerLocation))) (.Z (Math|Vector|BreakVector (Variables|Default|GetoldPlayerLocation)))) (Variables|Default|GetparallaxScrollingScaleZ)) (.Z (Math|Vector|BreakVector (Variables|Default|GetthisActorsLocation)))))))
      (Transformation|SetActorLocation _output_get_2 false false)
      (Variables|Default|SetoldPlayerLocation (Variables|Default|GetnewPlayerLocation)))))

(fn ConstructionScript)