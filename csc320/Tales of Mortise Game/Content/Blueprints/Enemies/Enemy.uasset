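; Side-scrolling enemy that patrols along X, flipping direction on hits or ledges and passing through other enemies.
; Tick drives movement, sprite facing and the health bar, and polls overlap with the first PlayerHero.
; An attacking player knocks the enemy back and damages it; otherwise the enemy knocks the player back and damages armor before health.
; Both use red or damage-color feedback with delayed damage, and the enemy is destroyed at zero health.
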(event EventBeginPlay
  (bind _charactermovement (Variables|Character|GetCharacterMovement))
  ;[1 1 1] Main
  (Variables|Default|SetscaleValue 1.0)
  (Math|Float|NegateFloat (Variables|Default|GetenemyDamage)
    (:%20%20
      (Variables|/Script/Engine.CharacterMovementComponent|SetMaxWalkSpeed _charactermovement (* (Variables|/Script/Engine.CharacterMovementComponent|GetMaxWalkSpeed _charactermovement) (Variables|Default|GetenemySpeed)))
      (bind _outactors (Actor|GetAllActorsOfClass "Enemy_C"))
      (for _array_element _outactors
        (Collision|IgnoreActorwhenMoving (Variables|Collision|GetCapsuleComponent) _array_element true)))))

(event Collision|EventHit
  (params (MyComp :type Primitive%20Component%20Object%20Reference) (Other :type Actor%20Object%20Reference) (OtherComp :type Primitive%20Component%20Object%20Reference) (bSelfMoved :type Boolean) (HitLocation :type Vector :default "0, 0, 0") (HitNormal :type Vector :default "0, 0, 0") (NormalImpulse :type Vector :default "0, 0, 0") (Hit :type Hit%20Result%20Structure%20%28by%20ref%29))
  ;[1 1 1] Handle Ledges
  (if (Variables|Default|GetcomingBackFromLedge)
    (Variables|Default|SetcomingBackFromLedge false)
    (else
      (Math|Float|NegateFloat (Variables|Default|GetscaleValue)))))

(event EventTick
  (params (DeltaSeconds :type Float%20%28single-precision%29))
  (bind _sprite (Variables|Default|GetSprite))
  ;[1 1 1] Determine When to Switch Direction
  (Utilities|FlowControl|Sequence
    (:then_0
      ;[1 1 1] Player Contact
      (bind _outactors (Actor|GetAllActorsOfClass "/Game/Blueprints/PlayerHero/PlayerHero.PlayerHero_C"))
      (Utilities|IsValid (Utilities|Array|Get(acopy) _outactors)
        (:Is%20Valid
          (if (and (Variables|/Game/Blueprints/PlayerHero/PlayerHero.PlayerHero_C|GetisAttacking (Utilities|Array|Get(acopy) _outactors)) (Collision|IsOverlappingActor (Utilities|Array|Get(acopy) _outactors) :!class /Script/Engine.Actor))
            (Utilities|HitbyPlayer (Utilities|Array|Get(acopy) _outactors))
            (elif (Collision|IsOverlappingActor (Utilities|Array|Get(acopy) _outactors) :!class /Script/Engine.Actor)
              (if (> (Variables|/Game/Blueprints/PlayerHero/PlayerHero.PlayerHero_C|GetplayerArmor (Utilities|Array|Get(acopy) _outactors)) 0.0)
                (Utilities|HitPlayerArmor (Utilities|Array|Get(acopy) _outactors))
                (else
                  (Utilities|HitPlayerHealth (Utilities|Array|Get(acopy) _outactors)))))))))
    (:then_1
      ;[1 1 1] Display Health
      (bind _asenemy_health (Utilities|Casting|CastToenemyHealth (UserInterface|GetUserWidgetObject (Variables|Default|GetWidget))))
      (Progress|SetPercent (Variables|/Game/UMG/enemyHealth.enemyHealth_C|GetEnemyHealthBar _asenemy_health) (/ (Variables|Default|GetenemyHealth) 1e+02)))
    (:then_2
      (Pawn|Input|AddMovementInput "1.000000, 0, 0" (Variables|Default|GetscaleValue) false)
      (Math|Float|CompareFloat (.X (Math|Vector|BreakVector (Transformation|GetVelocity))) 0.0
        (:>
          (Utilities|IsValid _sprite
            (:Is%20Valid
              (Transformation|SetRelativeRotation _sprite (Math|Rotator|MakeRotator 0.0 0.0 0.0) false false))))
        (:<
          (Utilities|IsValid _sprite
            (:Is%20Valid
              (Transformation|SetRelativeRotation _sprite (Math|Rotator|MakeRotator 0.0 0.0 1.8e+02) false false))))))))

(event EventOnWalkingOffLedge
  (params (PreviousFloorImpactNormal :type Vector%20%28by%20ref%29 :default "0, 0, 0") (PreviousFloorContactNormal :type Vector%20%28by%20ref%29 :default "0, 0, 0") (PreviousLocation :type Vector%20%28by%20ref%29 :default "0, 0, 0") (TimeDelta :type Float%20%28single-precision%29))
  (bind _returnvalue (Transformation|GetVelocity))
  (bind (_x _y _z) (Math|Vector|BreakVector _returnvalue))
  ;[1 1 1] Handle Ledges
  (bind _result (Math|Float|NegateFloat (Variables|Default|GetscaleValue))
    (:%20%20
      (Variables|/Script/Engine.MovementComponent|SetVelocity (Variables|Character|GetCharacterMovement) (Math|Vector|MakeVector (* _result _x 2.0) _y _z))
      (Variables|Default|SetcomingBackFromLedge true))))

(fn ConstructionScript)

(fn UpdateHealth
  (params (New%20Health :type Float%20%28single-precision%29))
  (if (> (+ New%20Health (Variables|Default|GetenemyHealth)) 1e+02)
    (Variables|Default|SetenemyHealth 1e+02)
    (elif (<= (+ New%20Health (Variables|Default|GetenemyHealth)) 0.0)
      (Variables|Default|SetenemyHealth 0.0)
      (Actor|DestroyActor)
      (else
        (Variables|Default|SetenemyHealth (+ New%20Health (Variables|Default|GetenemyHealth)))))))