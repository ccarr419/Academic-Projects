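; Loot chest that rolls its contents at BeginPlay and, when first opened, swaps to an open sprite and shows the loot to the player.
; CreateRandomLoot uses a weighted percentage roll to call a SetLootAs category routine, which sets exclusive type flags, name and amounts, often via a second tier roll.
; PrintChestLoot pushes a timed message to PlayerHero; nothing here adds the loot to the player.
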(event Custom|playerOpenChest
  ;[1 1 1] Open Chest and Get Loot
  (if (not (Variables|Default|GetchestIsOpen))
    (Rendering|Components|Sprite|SetSprite (Variables|Default|GetChestSprite) "/Game/Sprites/Objects/chestOpen_Sprite.chestOpen_Sprite")
    (Utilities|PrintChestLoot
      (:Exit
        (Variables|Default|SetchestIsOpen true)))))

(event EventBeginPlay
  ;[1 1 1] Determine the Contents of the Chest
  (Variables|Default|SetchestIsOpen false)
  (Utilities|CreateRandomLoot))

(fn ConstructionScript)