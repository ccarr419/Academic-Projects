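; NPC actor that turns its render component to face the player horizontally while the player is within its TalkRange.
; BeginPlay caches the actor's location with zero rotation and a fixed scale as StartLocation.
; Each Tick looks up the first PlayerHero and compares X positions, applying either a 180-degree flip or that cached transform.
; findOverlappingPlayer exposes the same TalkRange overlap test as a function.
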(event EventBeginPlay
  ;[1 1 1] Main
  (Variables|Default|SetstartLocation (Math|Transform|MakeTransform (Transformation|GetActorLocation) "0, 0, 0" "4.000000,4.000000,4.000000")))

(event EventTick
  (params (DeltaSeconds :type Float%20%28single-precision%29))
  (bind _rendercomponent (Variables|Default|GetRenderComponent))
  ;[1 1 1] Actor Orientation
  (bind _outactors (Actor|GetAllActorsOfClass "/Game/Blueprints/PlayerHero/PlayerHero.PlayerHero_C"))
  (if (Collision|IsOverlappingActor (Variables|Default|GetTalk%20Range) (Utilities|Array|Get(acopy) _outactors) :!class /Script/Engine.PrimitiveComponent)
    (if (>= (.X (Math|Vector|BreakVector (Transformation|GetActorLocation))) (.X (Math|Vector|BreakVector (Transformation|GetActorLocation (Utilities|Array|Get(acopy) _outactors)))))
      (Transformation|SetWorldTransform _rendercomponent (Math|Transform|MakeTransform (Transformation|GetWorldLocation _rendercomponent) "0,180.000000, 0" (Transformation|GetWorldScale _rendercomponent)) false false)
      (else
        (Transformation|SetWorldTransform _rendercomponent (Variables|Default|GetstartLocation) false false)))))

(fn ConstructionScript)