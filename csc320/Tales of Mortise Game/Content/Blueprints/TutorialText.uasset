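; TutorialText is an actor that shows its text render component only while the player hero overlaps it.
; The text starts hidden on BeginPlay.
; Every tick it fetches all PlayerHero actors, tests overlap against the first one, and sets visibility from the result, polling rather than using overlap events.
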(event EventBeginPlay
  (bind _output_get (Variables|Default|SetisVisible false))
  (Rendering|SetVisibility (Variables|Default|GetTextRender) _output_get false))

(event EventTick
  (params (DeltaSeconds :type Float%20%28single-precision%29))
  (bind _outactors (Actor|GetAllActorsOfClass "/Game/Blueprints/PlayerHero/PlayerHero.PlayerHero_C"))
  (if (Collision|IsOverlappingActor (Utilities|Array|Get(acopy) _outactors) :!class /Script/Engine.Actor)
    (Variables|Default|SetisVisible true)
    (else
      (Variables|Default|SetisVisible false)))
  (Rendering|SetVisibility (Variables|Default|GetTextRender) (Variables|Default|GetisVisible) false))

(fn ConstructionScript)