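; Ladder actor that lets the PlayerHero climb while Left Shift is held.
; Every Tick it finds the first PlayerHero and scans all Ladder actors for overlap, so each instance repeats the global check.
; It calls OnLadder on the hero unless they are swimming or jumped from climbing.
; Otherwise it clears IsOnLadder and calls ResetClimb when CheckIfResetIsNeeded returns true.
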(event EventBeginPlay
  ;[1 1 1] Main
  (Variables|Default|SetisOnLadder false)
  (Variables|Default|SetisByLadder false)
  (Variables|Default|SetneedsReset false))

(event EventTick
  (params (DeltaSeconds :type Float%20%28single-precision%29))
  (bind _returnvalue (Game|GetPlayerController 0))
  (bind _returnvalue_2 (Game|Player|IsInputKeyDown _returnvalue "LeftShift"))
  ;[1 1 1] Player is next to ladder
  (bind _outactors (Actor|GetAllActorsOfClass "/Game/Blueprints/PlayerHero/PlayerHero.PlayerHero_C"))
  (if (Utilities|IsValid (Utilities|Array|Get(acopy) _outactors))
    (bind _isonladder (Utilities|FindifOverlappingLadder (Utilities|Array|Get(acopy) _outactors))
      (:Exit
        (if (Math|Boolean|ANDBoolean _returnvalue_2 (not (Variables|/Game/Blueprints/PlayerHero/PlayerHero.PlayerHero_C|GetjumpedFromClimbing (Utilities|Array|Get(acopy) _outactors))) (not (Variables|/Game/Blueprints/PlayerHero/PlayerHero.PlayerHero_C|GetisSwimming (Utilities|Array|Get(acopy) _outactors))) _isonladder)
          (Variables|Default|SetisOnLadder true)
          (Default|OnLadder (Utilities|Array|Get(acopy) _outactors))
          (else
            (Variables|Default|SetisOnLadder false)
            (if (Utilities|CheckifResetIsNeeded _returnvalue_2 (Variables|/Game/Blueprints/PlayerHero/PlayerHero.PlayerHero_C|GetjumpedFromClimbing (Utilities|Array|Get(acopy) _outactors)))
              (Default|ResetClimb (Utilities|Array|Get(acopy) _outactors)))))))))

(fn ConstructionScript)