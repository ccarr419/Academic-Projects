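; Player hero character for a 2D Paper2D side-scroller, handling movement, animation, vitals, inventory and the pause and game-over screens.
; Ladder and water events poll overlap state in delayed loops, switching movement modes for climbing or swimming, with weaker jumps off either and oxygen loss underwater.
; Tick picks flipbooks from movement state and flips facing through control rotation.
; Activate greets overlapping NPCs and loots chests into health, armor or item counters.
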(event Custom|resetClimb
  ;[1 1 1] Climbing
  (Variables|Default|SetjumpedFromClimbing false))

(event Custom|Reset%20Camera
  (bind _sideviewcameracomponent (Variables|Camera|GetSideViewCameraComponent))
  (bind _sideviewcameracomponent_2 (Variables|Camera|GetSideViewCameraComponent))
  (bind _relativelocation (Variables|/Script/Engine.SceneComponent|GetRelativeLocation _sideviewcameracomponent))
  (bind _z (Math|Vector|BreakVector _relativelocation))
  (bind (_positivereturnvector _negativereturnvector) (Utilities|ResetCamera _z))
  ;[1 1 1] Move Camera
  (Math|Float|CompareFloat _z 0.0
    (:>
      (Transformation|SetRelativeLocationAndRotation _sideviewcameracomponent_2 _positivereturnvector "0, 0, 0" false false))
    (:<
      (Transformation|SetRelativeLocationAndRotation _sideviewcameracomponent_2 _negativereturnvector "0, 0, 0" false false))))

(event Custom|playerIsNearWaterSurface
  (params (isNearSurface :type Boolean))
  ;[1 1 1] Swimming
  (Variables|Default|SetcanJumpFromWater isNearSurface))

(event Custom|PlayerDied
  ;[1 1 1] Handle Player Death
  (bind _returnvalue (UserInterface|CreateWidget "/Game/UMG/GameOver.GameOver_C"))
  (Input|SetInputModeUIOnly (Game|GetPlayerController 0) _returnvalue "DoNotLock")
  (UserInterface|Viewport|AddtoViewport _returnvalue 0)
  (Utilities|FlowControl|Delay 3.0)
  (Game|QuitGame 0 "Quit"))

(event Custom|UpdateAnimation
  (bind _returnvalue (Transformation|GetVelocity))
  (bind _returnvalue_2 (Transformation|GetVelocity))
  (bind _charactermovement (Variables|Character|GetCharacterMovement))
  (bind _returnvalue_3 (AI|Components|NavMovement|IsFalling _charactermovement))
  (bind _returnvalue_4 (Math|Vector|VectorLength _returnvalue))
  (bind _z (Math|Vector|BreakVector _returnvalue_2))
  (bind _returnvalue_5 (> _returnvalue_4 0.0))
  (bind _returnvalue_6 (< _z -5e+02))
  (bind _returnvalue_7 (select _returnvalue_3 "/Game/Flipbooks/Hero/hero_jump.hero_jump" 0))
  (bind _returnvalue_8 (select _returnvalue_6 "/Game/Flipbooks/Hero/hero_falling.hero_falling" _returnvalue_7))
  ;[1 1 1] Handle Animation
  (Sprite|SetFlipbook (Variables|Default|GetSprite) (select (Variables|Default|GetisAttacking) "/Game/Flipbooks/Hero/hero_attack_default.hero_attack_default" (select (Variables|Default|GetisSwimming) "/Game/Flipbooks/Hero/hero_swim.hero_swim" (select (Utilities|IsValid _returnvalue_8) _returnvalue_8 (select (Variables|Default|GetisClimbing) (select _returnvalue_5 "/Game/Flipbooks/Hero/hero_climb.hero_climb" "/Game/Flipbooks/Hero/hero_climb_idle.hero_climb_idle") (select _returnvalue_5 "/Game/Flipbooks/Hero/hero_run.hero_run" "/Game/Flipbooks/Hero/hero_idle.hero_idle")))))))

(event Custom|addDamageColor
  (bind _sprite (Variables|Default|GetSprite))
  ;[1 1 1] Set Damage Color
  (Sprite|SetSpriteColor _sprite "(R=1.000000,G=0.000000,B=0.000000,A=1.000000)")
  (Utilities|FlowControl|Delay 0.75)
  (Sprite|SetSpriteColor _sprite "(R=1.000000,G=1.000000,B=1.000000,A=1.000000)"))

(event Custom|OnLadder
  (bind _returnvalue (Game|GetPlayerCharacter 0))
  (bind _charactermovement (Variables|/Script/Engine.Character|GetCharacterMovement _returnvalue))
  ;[1 1 1] Climbing
  (bind _isbyladder (Utilities|FindifPlayerIsbyLadder :!label _label)
    (:Exit
      (if _isbyladder
        (if (or (!= (Variables|Default|GetclimbScaleValue) 0.0) (not (Game|Player|IsInputKeyDown (Game|GetPlayerController 0) "SpaceBar")))
          (Pawn|Components|CharacterMovement|SetMovementMode _charactermovement "MOVE_Flying" 0) ; The player is climbing
          (Variables|/Script/Engine.MovementComponent|SetVelocity (Variables|Character|GetCharacterMovement) (Utilities|FindNewVelocity (Variables|Default|GetclimbVelocityVector))) ; Reset velocity to let player grab onto ladder
          (Utilities|FlowControl|Delay 0.1)
          (Variables|Default|SetisClimbing true) ; Loop back to check if the player got off the ladder
          (goto _label)
          (else
            _)))
      (Pawn|Components|CharacterMovement|SetMovementMode _charactermovement "MOVE_Walking" 0) ; The player is not climbing
      (Variables|Default|SetisClimbing false)
      (if (Variables|Default|GetisJumping)
        (CallFunction|JumpfromNonStanding) ; The player wants to jump
        (Variables|Default|SetjumpedFromClimbing true)))))

(event Custom|InWater
  (bind _returnvalue (Game|GetPlayerController 0))
  (bind _returnvalue_2 (Game|GetPlayerCharacter 0))
  (bind _returnvalue_3 (Game|Player|IsInputKeyDown _returnvalue "SpaceBar"))
  (bind _charactermovement (Variables|/Script/Engine.Character|GetCharacterMovement _returnvalue_2))
  ;[1 1 1] Swimming
  (bind _isinwater (Utilities|FindifPlayerIsinWater :!label _label)
    (:Exit
      (if _isinwater
        (Utilities|FlowControl|Delay (Utilities|FindPlayerSinkTime))
        (if (Math|Boolean|NANDBoolean (Variables|Default|GetcanJumpFromWater) _returnvalue_3)
          (Pawn|Components|CharacterMovement|SetMovementMode _charactermovement "MOVE_Swimming" 0)
          (Variables|/Script/Engine.MovementComponent|SetVelocity (Variables|Character|GetCharacterMovement) (Utilities|FindNewVelocity (Variables|Default|GetswimVelocityVector))) ; Reset velocity to let player grab onto ladder
          (Utilities|FlowControl|Delay 0.1)
          (Variables|Default|SetisSwimming true)
          (Utilities|UpdatePlayerOxygen
            (:Exit
              (goto _label)))
          (else
            _)))
      (Pawn|Components|CharacterMovement|SetMovementMode _charactermovement "MOVE_Walking" 0)
      (Variables|Default|SetisSwimming false)
      (if _returnvalue_3
        (if (Variables|Default|GetcanJumpFromWater)
          (CallFunction|JumpfromNonStanding))))))

(event EventDestroyed
  (CallFunction|PlayerDied))

(event EventTick
  (params (DeltaSeconds :type Float%20%28single-precision%29))
  ;[1 1 1] Tick - Updates animation
  (Utilities|FlowControl|Sequence
    (:then_0
      (CallFunction|UpdateAnimation)
      (Math|Float|CompareFloat (.X (Math|Vector|BreakVector (Variables|/Script/Engine.MovementComponent|GetVelocity (Pawn|GetMovementComponent)))) 0.0
        (:>
          (Pawn|SetControlRotation (Pawn|GetController) (Math|Rotator|MakeRotator 0.0 0.0 0.0) :!label _label))
        (:==
          (if (Variables|Default|GetbisMovingRight)
            (goto _label)
            (else
              (Pawn|SetControlRotation (Pawn|GetController) (Math|Rotator|MakeRotator 0.0 0.0 1.8e+02) :!label _label_2))))
        (:<
          (goto _label_2))))))

(event EventBeginPlay
  ;[1 1 1] Main
  (Utilities|FlowControl|Sequence
    (:then_0
      (Class|ActorComponent|SetIsReplicated (Variables|Default|GetSprite) true)
      (Variables|Default|SetCameraResetSpeed (/ (Variables|Default|GetCameraPanSpeed) 2.0))
      (Variables|Default|SetmaxJumpZVelocity (Variables|/Script/Engine.CharacterMovementComponent|GetJumpZVelocity (Variables|Character|GetCharacterMovement))))
    (:then_1
      (bind _returnvalue (UserInterface|CreateWidget "/Game/UMG/playerHUD.playerHUD_C" (Game|GetPlayerController 0)))
      (UserInterface|Viewport|AddtoViewport _returnvalue 0)
      (Variables|Default|SetplayerHealth 1e+02)
      (Variables|Default|SetplayerArmor 0.0)
      (Variables|Default|SetplayerOxygenLevel 1e+02)
      (Variables|Default|SetInventoryDisplayToggle true)
      (Variables|Default|SetresetGame false)
      (Math|Float|NegateFloat (Variables|Default|GetplayerDamage)))))

(event EventOnLanded
  (params (Hit :type Hit%20Result%20Structure%20%28by%20ref%29))
  ;[1 1 1] Handle Jump
  (Variables|/Script/Engine.CharacterMovementComponent|SetJumpZVelocity (Variables|Character|GetCharacterMovement) (Variables|Default|GetmaxJumpZVelocity))
  (Utilities|FlowControl|Sequence
    (:then_0
      (Variables|Default|SetisJumping false))
    (:then_1
      (Variables|Default|SetjumpedFromClimbing false))))

(event Input|ActionEvents|InputActionAttack
  (params (Key :type Key%20Structure :default "AnyKey"))
  ;[1 1 1] Attack
  (:Pressed
    (Variables|Default|SetisAttacking true)
    (Utilities|FlowControl|Delay 0.2)
    (Variables|Default|SetisAttacking false)))

(event Input|ActionEvents|InputActionJump
  (params (Key :type Key%20Structure :default "AnyKey"))
  ;[1 1 1] Handle Jump
  (:Pressed
    (if (Variables|Default|GetcanJumpFromWater)
      (Character|Jump)
      (Variables|Default|SetisJumping true)
      (else
        (Character|StopJumping :!label _label)
        (Variables|Default|SetisJumping false))))
  (:Released
    (goto _label)))

(event Input|AxisEvents|InputAxisMoveCamera
  (params (AxisValue :type Float%20%28single-precision%29))
  (bind _sideviewcameracomponent (Variables|Camera|GetSideViewCameraComponent))
  (bind _relativelocation (Variables|/Script/Engine.SceneComponent|GetRelativeLocation _sideviewcameracomponent))
  (bind _z (Math|Vector|BreakVector _relativelocation))
  ;[1 1 1] Move Camera
  (if (or (Utilities|FindifMoving) (Variables|Default|GetisSwimming))
    (CallFunction|ResetCamera)
    (else
      (Transformation|SetRelativeLocationAndRotation (Variables|Camera|GetSideViewCameraComponent) (Math|Vector|MakeVector 0.0 0.0 (select (Utilities|CheckCameraInput AxisValue _z) _z (Utilities|FindNewCameraZValue _z AxisValue))) "0, 0, 0" false false)
      (CallFunction|ResetCamera))))

(event Input|AxisEvents|InputAxisClimb
  (params (AxisValue :type Float%20%28single-precision%29))
  ;[1 1 1] Climbing
  (Variables|Default|SetclimbScaleValue AxisValue))

(event Input|AxisEvents|InputAxisMoveRight
  (params (AxisValue :type Float%20%28single-precision%29))
  ;[1 1 1] Handle movement
  (if (> AxisValue 0.0)
    (Variables|Default|SetbisMovingRight true)
    (elif (< AxisValue 0.0)
      (Variables|Default|SetbisMovingRight false)))
  (Pawn|Input|AddMovementInput "1.000000, 0, 0" AxisValue false)
  (Variables|Default|SetmoveScaleValue AxisValue))

(event Input|KeyboardEvents|X
  (params (Key :type Key%20Structure :default "AnyKey"))
  ;[1 1 1] Activate
  (:Pressed
    (if (not (Utilities|FindifMoving))
      (Utilities|FlowControl|Sequence
        (:then_0
          (bind _outactors (Actor|GetAllActorsOfClass "/Game/Blueprints/NPC/npcActor.npcActor_C"))
          (bind _array_element (Utilities|Array|ForEachLoopwithBreak _outactors :!label _label)
            (:LoopBody
              (if (Collision|IsOverlappingActor _array_element :!class /Script/Engine.Actor)
                (Variables|Default|SetprintMessage true)
                (Variables|Default|SetmessageText (Utilities|Text|ToText(String) (Utilities|String|Append "Hello, my name is " (Variables|/Game/Blueprints/NPC/npcActor.npcActor_C|GetnpcName _array_element))))
                (Utilities|FlowControl|Delay 3.0)
                (Variables|Default|SetprintMessage false)
                (Variables|Default|SetmessageText "")
                (goto _label Break)))))
        (:then_1
          (bind _outactors_2 (Actor|GetAllActorsOfClass "/Game/Blueprints/ChestContainer.ChestContainer_C"))
          (bind _array_element_2 (Utilities|Array|ForEachLoopwithBreak _outactors_2 :!label _label_2)
            (:LoopBody
              (if (and (Collision|IsOverlappingActor _array_element_2 :!class /Script/Engine.Actor) (not (Variables|/Game/Blueprints/ChestContainer.ChestContainer_C|GetchestIsOpen _array_element_2)))
                (Variables|Default|SetcanAddToInvetory true)
                (goto _label_2 Break)
                (else
                  (Variables|Default|SetcanAddToInvetory false))))
            (:Completed
              (Utilities|DistributeItemsfromChest _array_element_2))))))))

(event Input|KeyboardEvents|P
  (params (Key :type Key%20Structure :default "AnyKey"))
  (bind _returnvalue (Game|GetPlayerController 0))
  ;[1 1 1] Pause Menu
  (:Pressed
    (Utilities|IsValid (Variables|Default|GetPauseMenuReference)
      (:Is%20Valid
        _)
      (:Is%20Not%20Valid
        (bind _returnvalue_2 (UserInterface|CreateWidget "/Game/UMG/pauseMenu.pauseMenu_C"))
        (Variables|Default|SetPauseMenuReference _returnvalue_2)))
    (Input|SetInputModeUIOnly _returnvalue (Variables|Default|GetPauseMenuReference) "LockAlways")
    (UserInterface|Viewport|AddtoViewport (Variables|Default|GetPauseMenuReference) 0)
    (Game|SetGamePaused true)
    (Variables|/Script/Engine.PlayerController|SetbShowMouseCursor _returnvalue true)))

(event Input|KeyboardEvents|I
  (params (Key :type Key%20Structure :default "AnyKey"))
  ;[1 1 1] Toggle Inventory HUD
  (:Pressed
    (if (Variables|Default|GetInventoryDisplayToggle)
      (Variables|Default|SetInventoryDisplayToggle false)
      (else
        (Variables|Default|SetInventoryDisplayToggle true)))))

(fn ConstructionScript)

(fn JumpfromNonStanding
  (Variables|/Script/Engine.CharacterMovementComponent|SetJumpZVelocity (Variables|Character|GetCharacterMovement) (* (Variables|Default|GetmaxJumpZVelocity) 0.75))
  (Character|Jump))

(fn UpdateHealth
  (params (NewHealth :type Float%20%28single-precision%29))
  (if (> (+ NewHealth (Variables|Default|GetplayerHealth)) 1e+02)
    (Variables|Default|SetplayerHealth 1e+02)
    (elif (<= (+ NewHealth (Variables|Default|GetplayerHealth)) 0.0)
      (Variables|Default|SetplayerHealth 0.0)
      (CallFunction|PlayerDied)
      (else
        (Variables|Default|SetplayerHealth (+ NewHealth (Variables|Default|GetplayerHealth)))
        (Sprite|SetSpriteColor (Variables|Default|GetSprite) "(R=1.000000,G=1.000000,B=1.000000,A=1.000000)")))))

(fn UpdateArmor
  (params (NewArmor :type Float%20%28single-precision%29))
  (if (> (+ NewArmor (Variables|Default|GetplayerArmor)) 1e+02)
    (Variables|Default|SetplayerArmor 1e+02)
    (else
      (if (<= (+ NewArmor (Variables|Default|GetplayerArmor)) 0.0)
        (CallFunction|UpdateHealth (+ (+ NewArmor (Variables|Default|GetplayerArmor)) (Variables|Default|GetplayerArmor)))
        (Variables|Default|SetplayerArmor 0.0)
        (else
          (Variables|Default|SetplayerArmor (+ NewArmor (Variables|Default|GetplayerArmor)))))
      (Sprite|SetSpriteColor (Variables|Default|GetSprite) "(R=1.000000,G=1.000000,B=1.000000,A=1.000000)"))))